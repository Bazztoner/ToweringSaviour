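; BP_SnowTrap is a hero skill actor that places a temporary snow embankment and supplies its slow multiplier to a slow effector component.
; On BeginPlay it plays an attached skill sound, sets the multiplier and scales the mesh up with a timeline.
; A timer set to lifetime minus timeline length reverses that same timeline, shrinking the mesh and destroying the actor when the reverse finishes.
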(event Custom|DelayedDestroy
  (bind (_direction _sizetrack) (Timeline|GrowAnimation ReverseFromEnd)
    (:Update
      (Transformation|SetWorldScale3D (Variables|Default|GetS_Snow_Embankment_uhvjae0fa_lod5_Var1) _sizetrack))
    (:Finished
      (switch Utilities|FlowControl|Switch|SwitchonETimelineDirection _direction
        (:Backward
          (Actor|DestroyActor))))))

(event EventBeginPlay
  (Utilities|FlowControl|Sequence
    (:then_0
      (Audio|SpawnSoundAttached (Variables|Default|GetSkillSound) (Variables|Default|GetDefaultSceneRoot) "None" (Transformation|GetActorLocation) "0, 0, 0" "KeepRelativeOffset" true 1.0 1.0 0.0 0 0))
    (:then_1
      (Variables|/Game/Blueprints/Projectiles/HeroSkills/BP_SlowEffectorComponent.BP_SlowEffectorComponent_C|SetSlowMultiplier (Variables|Default|GetBP_SlowEffectorComponent) (Variables|Default|GetSlowMultiplier))
      (Utilities|Time|SetTimerbyEvent (delegate Custom|DelayedDestroy) (- (Variables|Default|GetLifeTime) (Components|Timeline|GetTimelineLength (Variables|Default|GetGrowAnimation)))))
    (:then_2
      (bind (_direction _sizetrack) (Timeline|GrowAnimation PlayFromStart)
        (:Update
          (Transformation|SetWorldScale3D (Variables|Default|GetS_Snow_Embankment_uhvjae0fa_lod5_Var1) _sizetrack))
        (:Finished
          (switch Utilities|FlowControl|Switch|SwitchonETimelineDirection _direction
            (:Backward
              (Actor|DestroyActor))))))))

(fn ConstructionScript)