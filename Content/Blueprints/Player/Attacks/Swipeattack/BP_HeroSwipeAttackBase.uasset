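; Base Blueprint for the hero's swipe attack, which spawns a projectile and enforces a cooldown between uses.
; TrySwipeAttack fails while on cooldown; otherwise it spawns the SwipeAttackProjectile class at the given position and direction, restarts the cooldown and returns true.
; Tick counts the timer up to the cooldown length to re-enable the attack, and GetCooldownValues exposes max, current and fractional progress.
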(event EventTick
  (params (DeltaSeconds :type Float%20%28single-precision%29))
  (if (Variables|Default|GetbOnCooldown)
    (Variables|Default|Set_currentCooldown (Math|Float|Clamp(Float) (+ DeltaSeconds (Variables|Default|Get_currentCooldown)) 0.0 (Variables|Default|GetCooldown)))
    (if (== (Variables|Default|Get_currentCooldown) (Variables|Default|GetCooldown))
      (Variables|Default|SetbOnCooldown false))))

(event EventBeginPlay
  (Variables|Default|Set_currentCooldown (Variables|Default|GetCooldown)))

(fn TrySwipeAttack
  (params (Position :type Vector) (Direction :type Rotator))
  (if (Variables|Default|GetbOnCooldown)
    (return false)
    (else
      (Utilities|FlowControl|Sequence
        (:then_0
          (Game|SpawnActorfromClass (Variables|Default|GetSwipeAttackProjectile) (Math|Transform|MakeTransform Position Direction "1.000000,1.000000,1.000000") "AlwaysSpawn" 0 0))
        (:then_1
          (Variables|Default|Set_currentCooldown 0.0)
          (Variables|Default|SetbOnCooldown true)
          (return true))))))

(fn GetCooldownValues
  (return (Variables|Default|GetCooldown) (Variables|Default|Get_currentCooldown) (/ (Variables|Default|Get_currentCooldown) (Variables|Default|GetCooldown))))