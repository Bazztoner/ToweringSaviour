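; Wave manager that spawns enemies from BP_WaveClass objects near random SpawnPoints, capped by MaxActiveEnemies, and registers itself with the player character.
; Kills update game-instance counters, grant mana with floating text for player kills, and on wave completion trigger a delayed advance plus a new randomly sized wave.
; FindClosestEnemy returns the nearest active enemy within player attack range.
; The setup chain for spawn points, starting waves and spawn timer is unwired.
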(event Custom|FinishWave
  (Development|PrintString "GET READY FOR NEXT WAVE" false false "(R=1.000000,G=0.184895,B=0.000000,A=1.000000)" (Variables|Default|GetWaveChangeDelay))
  (Utilities|FlowControl|Delay (Variables|Default|GetWaveChangeDelay))
  (CallFunction|ChangetoNextWave)
  (CallFunction|AddNextWave))

(event Custom|EnemySpawnHandler
  (CallFunction|SpawnEnemy))

(event EventBeginPlay
  (Utilities|FlowControl|DelayUntilNextTick)
  (Variables|/Game/Blueprints/Characters/Frontline/Hero/BP_HeroBase.BP_HeroBase_C|SetWaveManager (Variables|/Game/Blueprints/Player/BP_PlayerController.BP_PlayerController_C|GetPlayerCharacter (CallFunction|GetFrontlinePlayerController)) self))

(fn ConstructionScript)

(fn OnKilledEnemy
  (params (EnemyKilled :type BP%20Enemy%20Base%20Object%20Reference) (KilledByPlayer :type Boolean))
  (bind _gameinstancefrontline (CallFunction|GetFrontlineGameInstance))
  (Utilities|FlowControl|Sequence
    (:then_0
      (LocalVariables|SetEnemy EnemyKilled)
      (LocalVariables|SetByPlayer KilledByPlayer))
    (:then_1
      (Utilities|IsValid (LocalVariables|GetEnemy)
        (:Is%20Valid
          (Utilities|Array|RemoveItem (Variables|Default|GetActiveEnemies) (LocalVariables|GetEnemy)))))
    (:then_2
      (if (LocalVariables|GetByPlayer)
        (CallFunction|OnPlayerKilledEnemy (LocalVariables|GetEnemy))))
    (:then_3
      (Math|Integer|IncrementInt (Variables|/Game/Blueprints/Managers/GI_Frontline.GI_Frontline_C|GetEnemiesKilledTotal _gameinstancefrontline)
        (:%20%20
          (Math|Integer|IncrementInt (Variables|/Game/Blueprints/Managers/GI_Frontline.GI_Frontline_C|GetEnemiesKilledWave _gameinstancefrontline)))))
    (:then_4
      (bind _wave_clear (Default|OnEnemyDeath (Utilities|Array|Get(acopy) (Variables|Default|GetAllWaves) (Variables|Default|GetCurrentWave))))
      (if _wave_clear
        (CallFunction|FinishWave)))))

(fn OnPlayerKilledEnemy
  (params (EnemyKilled :type BP%20Enemy%20Base%20Object%20Reference))
  (Default|OnEnemyKilled (CallFunction|GetFrontlinePlayerController) (Variables|/Game/Blueprints/Characters/Frontline/Enemy/BP_EnemyBase.BP_EnemyBase_C|GetManaGrantedOnKill EnemyKilled))
  (Game|SpawnActorfromClass "/Game/Blueprints/Misc/BP_3DText.BP_3DText_C" (Math|Transform|MakeTransform (+ (Transformation|GetActorLocation EnemyKilled) "0,0,200.000000") "0, 0, 0" "1.000000,1.000000,1.000000") "AlwaysSpawn" "OverrideRootScale" 0 (Utilities|Text|ToText(String) (Utilities|String|Append "+" (Utilities|String|ToString(Integer) (Variables|/Game/Blueprints/Characters/Frontline/Enemy/BP_EnemyBase.BP_EnemyBase_C|GetManaGrantedOnKill EnemyKilled)))) "(R=0.000000,G=0.925979,B=1.000000,A=1.000000)" 0))

(fn SpawnEnemy
  (bind _output_get (LocalVariables|SetWaveObject (Utilities|Array|Get(acopy) (Variables|Default|GetAllWaves) (Variables|Default|GetCurrentWave))))
  (bind _space_available (Default|GetEnemyAmount _output_get))
  (if (and _space_available (< (Utilities|Array|Length (Variables|Default|GetActiveEnemies)) (Variables|Default|GetMaxActiveEnemies)))
    (bind _enemyclass (Default|GetEnemy (LocalVariables|GetWaveObject)))
    (bind (_randomlocation _return_value_rotation _return_value_scale) (CallFunction|GetRandomSpawnPoint))
    (bind _returnvalue (Game|SpawnActorfromClass _enemyclass (Math|Transform|MakeTransform _randomlocation _return_value_rotation _return_value_scale) "AlwaysSpawn" "SelectDefaultAtRuntime" 0 self 0))
    (Utilities|Array|Add (Variables|Default|GetActiveEnemies) _returnvalue)
    (Default|AddEnemy (LocalVariables|GetWaveObject) _returnvalue)
    (Utilities|Array|SetArrayElem (Variables|Default|GetAllWaves) (Variables|Default|GetCurrentWave) (LocalVariables|GetWaveObject) true)))

(fn GetRandomSpawnPoint
  (bind _spawnpoints (Variables|Default|GetSpawnPoints))
  (bind _outitem (Utilities|Array|Random _spawnpoints))
  (bind _returnvalue (Transformation|GetActorTransform _outitem))
  (bind _randomlocation (Class|NavigationSystemV1|GetRandomLocationinNavigableRadius (.location _returnvalue) 5e+02 0 0))
  (return _randomlocation (.rotation _returnvalue) (.scale _returnvalue)))

(fn FindClosestEnemy
  (bind _frontline_player_controller (CallFunction|GetFrontlinePlayerController))
  (bind _activeenemies (Variables|Default|GetActiveEnemies))
  (bind _playercharacter (Variables|/Game/Blueprints/Player/BP_PlayerController.BP_PlayerController_C|GetPlayerCharacter _frontline_player_controller))
  (bind _returnvalue (Transformation|GetActorLocation _playercharacter))
  (bind (_distance _returnvalue_2) (Actor|FindNearestActor _returnvalue _activeenemies))
  (Utilities|IsValid _frontline_player_controller
    (:Is%20Valid
      (bind _asbp_enemy_base (Utilities|Casting|CastToBP_EnemyBase _returnvalue_2))
      (if (>= (Variables|/Game/Blueprints/Characters/Frontline/Hero/BP_HeroBase.BP_HeroBase_C|GetAttackRange _playercharacter) _distance)
        (return _asbp_enemy_base)))))

(fn CreateNewWave
  (params (WaveNumber :type Integer) (EnemyAmount :type Integer))
  (bind _returnvalue (Game|SpawnActorfromClass "/Game/Blueprints/Managers/WaveSystem/BP_WaveClass.BP_WaveClass_C" (Math|Transform|MakeTransform "666.000000,666.000000,666.000000" "0, 0, 0" "1.000000,1.000000,1.000000") "AlwaysSpawn" "OverrideRootScale" 0 WaveNumber 0))
  (Variables|/Game/Blueprints/Managers/WaveSystem/BP_WaveClass.BP_WaveClass_C|SetEnemyData _returnvalue (Utilities|Struct|MakeSTRUCT_WaveData (Math|Integer|Clamp(Integer) EnemyAmount 1 100) (Utilities|Map|MakeMap "/Game/Blueprints/Characters/Frontline/Enemy/BP_EnemyWeak.BP_EnemyWeak_C" 50 "/Game/Blueprints/Characters/Frontline/Enemy/BP_EnemyMid.BP_EnemyMid_C" 35 "/Game/Blueprints/Characters/Frontline/Enemy/BP_EnemyStrong.BP_EnemyStrong_C" 15)))
  (Utilities|Array|AddUnique (Variables|Default|GetAllWaves) _returnvalue))

(fn AddNextWave
  (bind _allwaves (Variables|Default|GetAllWaves))
  (bind _enemies_amount (Default|GetEnemyAmount (Utilities|Array|Get(acopy) _allwaves (Utilities|Array|LastIndex _allwaves))))
  (CallFunction|CreateNewWave (Utilities|Array|Length _allwaves) (+ _enemies_amount (Math|Random|RandomIntegerinRange -5 8))))

(fn CreateStartingWaves
  (CallFunction|CreateNewWave 1 10)
  (CallFunction|CreateNewWave 2 13)
  (CallFunction|CreateNewWave 3 17)
  (CallFunction|CreateNewWave 4 22)
  (CallFunction|CreateNewWave 5 16))

(fn ChangetoNextWave
  (bind _result (Math|Integer|IncrementInt (Variables|Default|GetCurrentWave))
    (:%20%20
      (bind _enemies_amount (Default|GetEnemyAmount (Utilities|Array|Get(acopy) (Variables|Default|GetAllWaves) _result)))
      (Default|ChangeWave (CallFunction|GetFrontlineGameInstance) (Variables|/Game/Blueprints/Managers/WaveSystem/BP_WaveClass.BP_WaveClass_C|GetWaveNumber (Utilities|Array|Get(acopy) (Variables|Default|GetAllWaves) _result)) _enemies_amount)
      (if (> (Variables|Default|GetCurrentWave) 0)
        (Audio|PlaySound2D "/Game/Sound/SFX/UI/NewWaveIncoming_Cue.NewWaveIncoming_Cue" 1.0 1.0 0.0 0 0)))))