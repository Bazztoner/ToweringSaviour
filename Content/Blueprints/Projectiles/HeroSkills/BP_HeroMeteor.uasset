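; BP_HeroMeteor is a hero skill meteor projectile that deals area damage to enemies on impact.
; It plays an attached launch sound on spawn, which stops when the meteor is destroyed.
; On Hit, a zero-length multi-sphere trace on the Camera channel finds actors within Radius, ignoring the Instigator, and damages those that cast to BP_EnemyBase.
; It then spawns a pooled explosion effect, plays the hit sound and destroys itself.
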(event EventBeginPlay
  (bind _sphere (Variables|Default|GetSphere))
  (Audio|SpawnSoundAttached (Variables|Default|GetLaunchSound) _sphere "None" (Transformation|GetWorldLocation _sphere) "0, 0, 0" "KeepRelativeOffset" true 1.0 1.0 0.0 0 0))

(event Collision|EventHit
  (params (MyComp :type Primitive%20Component%20Object%20Reference) (Other :type Actor%20Object%20Reference) (OtherComp :type Primitive%20Component%20Object%20Reference) (bSelfMoved :type Boolean) (HitLocation :type Vector :default "0, 0, 0") (HitNormal :type Vector :default "0, 0, 0") (NormalImpulse :type Vector :default "0, 0, 0") (Hit :type Hit%20Result%20Structure%20%28by%20ref%29))
  (bind _outhits (Collision|MultiSphereTraceByChannel HitLocation HitLocation (Variables|Default|GetRadius) "TraceTypeQuery2" false (Utilities|Array|MakeArray (Variables|Actor|GetInstigator)) "None"))
  (for _array_element _outhits
    (bind _asbp_enemy_base (Utilities|Casting|CastToBP_EnemyBase (.HitActor (Collision|BreakHitResult _array_element))))
    (Game|Damage|ApplyDamage _asbp_enemy_base (Variables|Default|GetDamage) 0 0))
  (Niagara|SpawnSystematLocation "/Game/Art/Particles/PS_MeteorExplosion.PS_MeteorExplosion" HitLocation "0, 0, 0" "1.000000,1.000000,1.000000" true true "AutoRelease")
  (Audio|PlaySoundatLocation (Variables|Default|GetHitSound) HitLocation "0, 0, 0" 1.0 1.0 0.0 0 0 0 0)
  (Actor|DestroyActor))

(fn ConstructionScript)