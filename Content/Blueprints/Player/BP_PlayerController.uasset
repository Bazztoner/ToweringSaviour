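; Player controller that spawns and possesses the hero class from the game instance, replacing the default pawn, and sets a small portrait window.
; Taps grant a timed attack-speed boost that restarts on each tap.
; Swipes become attack directions toward left, right or top spawn points found by display name.
; It relays skill and kill events to the hero and projects mouse or Android touch input onto the hero's ground plane.
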(event Custom|OnAttackSpeedIncrease
  (Default|ModifyAttackSpeed (Variables|Default|GetPlayerCharacter) false))

(event Custom|OnHeroSwiped
  (params (Direction :type Vector%202D%20Structure))
  (bind _finaldirection (CallFunction|ConvertSwipeDirection Direction))
  (Default|SpawnSwipeAttack (Variables|Default|GetPlayerCharacter) _finaldirection))

(event Custom|OnHeroTapped
  (Default|ModifyAttackSpeed (Variables|Default|GetPlayerCharacter) true)
  (Utilities|FlowControl|Sequence
    (:then_0
      (if (Utilities|Time|IsValidTimerHandle (Variables|Default|GetAttackSpeedTimer))
        (Utilities|Time|ClearandInvalidateTimerbyHandle (Variables|Default|GetAttackSpeedTimer))))
    (:then_1
      (bind _returnvalue (Utilities|Time|SetTimerbyEvent (delegate Custom|OnAttackSpeedIncrease) (Variables|Default|GetIncreaseAttackSpeedDuration)))
      (Variables|Default|SetAttackSpeedTimer _returnvalue))))

(event EventBeginPlay
  (Utilities|FlowControl|Sequence
    (:then_0
      (bind _herocharacterpicked (Default|GetPlayerCharacter (CallFunction|GetFrontlineGameInstance)))
      (bind _returnvalue (Game|SpawnActorfromClass _herocharacterpicked (Transformation|GetActorTransform (Pawn|GetControlledPawn)) "AlwaysSpawn" 0 0))
      (bind _output_get (Variables|Default|SetPlayerCharacter _returnvalue))
      (Actor|DestroyActor (Pawn|GetControlledPawn))
      (Pawn|Possess _output_get))
    (:then_1
      (bind _returnvalue_2 (Settings|GetGameUserSettings))
      (Class|GameUserSettings|SetFullscreenMode _returnvalue_2 "Windowed")
      (Class|GameUserSettings|SetScreenResolution _returnvalue_2 (Utilities|Struct|MakeIntPoint 375 667))
      (Class|GameUserSettings|ApplyResolutionSettings _returnvalue_2 false))
    (:then_2
      (Input|SetInputModeGameandUI self 0 "DoNotLock" false false))))

(fn ConstructionScript)

(fn ConvertSwipeDirection
  (params (Direction :type Vector%202D%20Structure))
  (bind (_x _y) (Math|Vector2D|BreakVector2D Direction))
  (Utilities|FlowControl|Sequence
    (:then_0
      (bind _outactors (Actor|GetAllActorsOfClass "/Game/Blueprints/Managers/SpawnPoint.SpawnPoint_C"))
      (LocalVariables|SetSpawnPoints _outactors))
    (:then_1
      (LocalVariables|SetTopSwipe (< _y 0.0)))
    (:then_2
      (LocalVariables|SetRightSwipe (> _x 0.0)))
    (:then_3
      (LocalVariables|SetLeftSwipe (< _x 0.0)))
    (:then_4
      (if (LocalVariables|GetLeftSwipe)
        (bind _array_element (Utilities|Array|ForEachLoopwithBreak (LocalVariables|GetSpawnPoints) :!label _label)
          (:LoopBody
            (if (Utilities|Enum|Equal(Enum) (Utilities|GetDisplayName _array_element) "LeftSP")
              (LocalVariables|SetChosenPoint (Transformation|GetActorLocation _array_element))
              (goto _label Break))))
        (elif (LocalVariables|GetRightSwipe)
          (bind _array_element_2 (Utilities|Array|ForEachLoopwithBreak (LocalVariables|GetSpawnPoints) :!label _label_2)
            (:LoopBody
              (if (Utilities|Enum|Equal(Enum) (Utilities|GetDisplayName _array_element_2) "RightSP")
                (LocalVariables|SetChosenPoint (Transformation|GetActorLocation _array_element_2))
                (goto _label_2 Break))))
          (elif (LocalVariables|GetTopSwipe)
            (bind _array_element_3 (Utilities|Array|ForEachLoopwithBreak (LocalVariables|GetSpawnPoints) :!label _label_3)
              (:LoopBody
                (if (Utilities|Enum|Equal(Enum) (Utilities|GetDisplayName _array_element_3) "TopSP")
                  (LocalVariables|SetChosenPoint (Transformation|GetActorLocation _array_element_3))
                  (goto _label_3 Break))))))))
    (:then_5
      (return (Math|Conversions|ToVector2D(Vector) (Class|KismetMathLibrary|VectorNormal2D (- (LocalVariables|GetChosenPoint) (Transformation|GetActorLocation (Variables|Default|GetPlayerCharacter))) 0.0001))))))

(fn GetMouseorFingerPosition
  (bind (_worldlocation _worlddirection) (Game|Player|ConvertMouseLocationToWorldSpace))
  (bind (_locationx _locationy) (Class|PlayerController|GetInputTouchState "Touch1"))
  (bind (_worldlocation_2 _worlddirection_2) (Class|PlayerController|DeprojectScreenPositiontoWorld _locationx _locationy))
  (Utilities|FlowControl|Sequence
    (:then_0
      (if (Utilities|Enum|Equal(Enum) (Game|GetPlatformName) "Android")
        (LocalVariables|SetWorldLocation _worldlocation_2)
        (LocalVariables|SetWorldDirection _worlddirection_2)
        (elif (not (Variables|/Game/Blueprints/Widgets/Frontline/HUD_Frontline_Skills.HUD_Frontline_Skills_C|GetMouseCaptured (Variables|/Game/Blueprints/Characters/Frontline/Hero/BP_HeroBase.BP_HeroBase_C|GetHUDSkills (Variables|Default|GetPlayerCharacter))))
          (LocalVariables|SetWorldLocation _worldlocation)
          (LocalVariables|SetWorldDirection _worlddirection))))
    (:then_1
      (return (.Intersection (Class|KismetMathLibrary|LinePlaneIntersectionOriginNormal (LocalVariables|GetWorldLocation) (+ (LocalVariables|GetWorldLocation) (* (LocalVariables|GetWorldDirection) 5e+05)) (Transformation|GetActorLocation (Variables|Default|GetPlayerCharacter)) "0, 0,1.000000"))))))

(fn OnEnemyKilled
  (params (ManaEarned :type Integer))
  (Default|OnEnemyKilled (Variables|Default|GetPlayerCharacter) ManaEarned))

(fn OnSkillButtonStart
  (params (SkillID :type Integer))
  (Default|OnSkillStart (Variables|Default|GetPlayerCharacter) SkillID))

(fn OnSkillButtonRelease
  (params (SkillID :type Integer))
  (Default|OnSkillEnd (Variables|Default|GetPlayerCharacter) SkillID))

(fn CheckSkillAvailable
  (params (SkillID :type Integer))
  (bind _playercharacter (Variables|Default|GetPlayerCharacter))
  (Utilities|IsValid _playercharacter
    (:Is%20Valid
      (bind _available (Default|CheckSkillAvailable _playercharacter SkillID))
      (return _available))))