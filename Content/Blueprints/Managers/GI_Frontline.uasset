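; GI_Frontline is the game instance that holds hero selection and wave progress for a wave-based game.
; GetPlayerCharacter returns the picked hero, or randomly one of Ninja, Mage Serath or Annihilator while RandomCharacter is set; PickCharacter clears that flag.
; ChangeWave stores the new wave and enemy count and clears that wave's kills.
; RestartGame zeroes all wave and kill counters but keeps the hero choice.
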(fn GetPlayerCharacter
  (if (Variables|Default|GetRandomCharacter)
    (return (Utilities|Select :Index (Math|Random|RandomIntegerinRange 0 2) :Option%200 "/Game/Blueprints/Characters/Frontline/Hero/BP_HeroNinja.BP_HeroNinja_C" :Option%201 "/Game/Blueprints/Characters/Frontline/Hero/BP_HeroMageSerath.BP_HeroMageSerath_C" :Option%202 "/Game/Blueprints/Characters/Frontline/Hero/BP_HeroAnnihilator.BP_HeroAnnihilator_C"))
    (else
      (return (Variables|Default|GetHeroCharacterPicked)))))

(fn ChangeWave
  (params (CurrentWave :type Integer) (EnemiesInWave :type Integer))
  (Variables|Default|SetCurrentWave CurrentWave)
  (Variables|Default|SetEnemiesInWave EnemiesInWave)
  (Variables|Default|SetEnemiesKilledWave 0))

(fn RestartGame
  (bind _output_get (Variables|Default|SetEnemiesKilledTotal 0))
  (bind _output_get_2 (Variables|Default|SetEnemiesKilledWave _output_get))
  (bind _output_get_3 (Variables|Default|SetEnemiesInWave _output_get_2))
  (Variables|Default|SetCurrentWave _output_get_3))

(fn PickCharacter
  (params (HeroCharacterPicked :type BP%20Hero%20Base%20Class%20Reference))
  (Variables|Default|SetRandomCharacter false)
  (Variables|Default|SetHeroCharacterPicked HeroCharacterPicked))