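; Base player hero for the Frontline mode that auto-targets the closest enemy via the wave manager and opens the lose screen on death.
; Tick updates target, attack flag and screen-following HP HUD.
; BeginPlay builds skills and both attacks as components from container-supplied classes, creates HUDs and starts timed mana regeneration, topped up by kills.
; Touches starting on the hero become taps or swipes by screen distance and go to the player controller.
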(event Custom|RegenerateMana
  (CallFunction|ModifyManaValues true (* (Variables|Default|GetManaPerSecond) (Variables|Default|GetManaRegenTick))))

(event Custom|TapDown
  (params (FingerIndex :type ETouchIndex%20Enum :default "Touch1") (TouchedActor :type Actor%20Object%20Reference))
  (Variables|Default|SetbIsTapped true))

(event EventBeginPlay
  (Utilities|FlowControl|Sequence
    (:then_0
      (|CallParentFunction)
      (Variables|Default|SetCurrentAttackSpeed (Variables|Default|GetDefaultAttackAnimSpeed))
      (bind _asbp_player_controller (Utilities|Casting|CastToBP_PlayerController (Game|GetPlayerController 0)))
      (Variables|Default|SetPlayerController _asbp_player_controller)
      (CallFunction|GetAllSkills)
      (CallFunction|GetCurrentAttacks))
    (:then_1
      (bind _returnvalue (UserInterface|CreateWidget "/Game/Blueprints/Widgets/Frontline/HUD_Frontline_Skills.HUD_Frontline_Skills_C" (Game|GetPlayerController 0)))
      (bind _output_get (Variables|Default|SetHUDSkills _returnvalue))
      (UserInterface|Viewport|AddtoViewport _output_get 0)
      (bind _returnvalue_2 (UserInterface|CreateWidget "/Game/Blueprints/Widgets/Frontline/HUD_Frontline_Player.HUD_Frontline_Player_C" (Game|GetPlayerController 0)))
      (bind _output_get_2 (Variables|Default|SetHUDHP _returnvalue_2))
      (UserInterface|Viewport|AddtoViewport _output_get_2 1))
    (:then_2
      (EventDispatchers|BindEventtoOnInputTouchBegin (delegate Custom|TapDown)))
    (:then_3
      (Utilities|Time|SetTimerbyEvent (delegate Custom|RegenerateMana) (Variables|Default|GetManaRegenTick) true))))

(event EventTick
  (params (DeltaSeconds :type Float%20%28single-precision%29))
  (CallFunction|CheckTarget)
  (CallFunction|Attack)
  (CallFunction|HandleHUDPosition))

(event Input|TouchEvents|InputTouch
  (params (Location :type Vector) (FingerIndex :type ETouchIndex%20Enum))
  (:Released
    (if (Variables|Default|GetbIsTapped)
      (bind (_hasswiped _direction) (CallFunction|CheckSwipe))
      (Utilities|FlowControl|Sequence
        (:then_0
          (Variables|Default|SetbIsTapped false))
        (:then_1
          (if _hasswiped
            (CallFunction|OnSwipe (Math|Conversions|ToVector2D(Vector) _direction))
            (else
              (CallFunction|OnActorTapped))))))))

(fn ConstructionScript
  (|CallParentFunction))

(fn HandleScreenSize
  (bind _returnvalue (Viewport|GetViewportSize))
  (Camera|SetFieldOfView (Variables|Default|GetCamera) (* (/ (.x _returnvalue) (.y _returnvalue)) 9e+01)))

(fn Attack
  (Variables|Default|SetbIsAttacking (Utilities|IsValid (Variables|Default|GetCurrentTarget))))

(fn CheckTarget
  (Utilities|FlowControl|Sequence
    (:then_0
      (Utilities|IsValid (Variables|Default|GetWaveManager)
        (:Is%20Not%20Valid
          (bind _returnvalue (Actor|GetActorOfClass "/Game/Blueprints/Managers/BP_WaveManager.BP_WaveManager_C"))
          (Utilities|IsValid _returnvalue
            (:Is%20Valid
              (Variables|Default|SetWaveManager _returnvalue))
            (:Is%20Not%20Valid
              (bind _returnvalue_2 (Game|SpawnActorfromClass "/Game/Blueprints/Managers/BP_WaveManager.BP_WaveManager_C" (Math|Transform|MakeTransform "616.000000,616.000000,616.000000" "0, 0, 0" "1.000000,1.000000,1.000000") "AlwaysSpawn" "OverrideRootScale" 0 0))
              (Variables|Default|SetWaveManager _returnvalue_2))))))
    (:then_1
      (bind _enemy (Default|FindClosestEnemy (Variables|Default|GetWaveManager)))
      (Variables|Default|SetCurrentTarget _enemy))))

(fn SpawnAutoattack
  (bind _projspawnpos (Variables|Default|GetProjSpawnPos))
  (bind _returnvalue (Transformation|GetWorldLocation _projspawnpos))
  (if (Utilities|IsValid (Variables|Default|GetCurrentTarget))
    (Game|SpawnActorfromClass (Variables|/Game/Blueprints/Player/Attacks/Autoattack/BP_HeroAutoAttackBase.BP_HeroAutoAttackBase_C|GetAutoattackProjectile (Variables|Default|GetAutoattack)) (Math|Transform|MakeTransform _returnvalue (Math|Conversions|RotationFromXVector (Math|Vector|Normalize (- (Transformation|GetWorldLocation (Variables|/Script/Engine.Actor|GetRootComponent (Variables|Default|GetCurrentTarget))) _returnvalue))) "1.000000,1.000000,1.000000") "Undefined" "SelectDefaultAtRuntime" 0 (Variables|Default|GetCurrentTarget) 0)
    (Audio|PlaySoundatLocation (Variables|Default|GetAutoattackSound) (Transformation|GetActorLocation) "0, 0, 0" 1.0 1.0 0.0 0 0 0 0)))

(fn SpawnSwipeAttack
  (params (Direction :type Vector%202D%20Structure))
  (bind _returnvalue (Math|Conversions|ToVector(Vector2D) Direction))
  (bind (_x _y) (Math|Vector2D|BreakVector2D Direction))
  (if (not (and (== _x 0.0) (== _y 0.0)))
    (bind _attacksuccessful (Default|TrySwipeAttack (Variables|Default|GetSwipeAttack) (Transformation|GetWorldLocation (Variables|Default|GetProjSpawnPos)) (Math|Conversions|RotationFromXVector (Math|Vector|MakeVector (.x _returnvalue) (.y _returnvalue) 0.0))))
    (if _attacksuccessful
      (Audio|PlaySoundatLocation (Variables|Default|GetSwipeAttackSound) (Transformation|GetActorLocation) "0, 0, 0" 1.0 1.0 0.0 0 0 0 0))))

(fn ModifyAttackSpeed
  (params (Increase :type Boolean))
  (if Increase
    (Variables|Default|SetCurrentAttackSpeed (Variables|Default|GetFastAttackAnimSpeed))
    (else
      (Variables|Default|SetCurrentAttackSpeed (Variables|Default|GetDefaultAttackAnimSpeed)))))

(fn OnActorTapped
  (Default|OnHeroTapped (Variables|Default|GetPlayerController)))

(fn CheckSwipe
  (bind _playercontroller (Variables|Default|GetPlayerController))
  (bind _capsulecomponent (Variables|Default|GetCapsuleComponent))
  (bind (_locationx _locationy) (Class|PlayerController|GetInputTouchState _playercontroller "Touch1"))
  (bind _returnvalue (Transformation|GetWorldLocation _capsulecomponent))
  (bind _returnvalue_2 (Math|Vector2D|MakeVector2D _locationx _locationy))
  (bind _screenposition (Class|GameplayStatics|ProjectWorldtoScreen _playercontroller _returnvalue false))
  (LocalVariables|SetDistance (Math|Vector|Distance2D(Vector) _screenposition _returnvalue_2))
  (bind _output_get (LocalVariables|SetDirectionVector (Class|KismetMathLibrary|VectorNormal2D (Math|Vector|GetUnitDirection(Vector) (Math|Conversions|ToVector(Vector2D) _screenposition) (Math|Conversions|ToVector(Vector2D) _returnvalue_2)) 0.0001)))
  (return (>= (LocalVariables|GetDistance) (Variables|Default|GetSwipeStartDistance)) _output_get))

(fn OnSwipe
  (params (SwipeDirection :type Vector%202D%20Structure))
  (Default|OnHeroSwiped (Variables|Default|GetPlayerController) (Class|KismetMathLibrary|ToRounded2D SwipeDirection)))

(fn ModifyManaValues
  (params (Increase :type Boolean) (Amount :type Float%20%28double-precision%29))
  (Utilities|FlowControl|Sequence
    (:then_0
      (if Increase
        (LocalVariables|SetMultiplier 1.0)
        (else
          (LocalVariables|SetMultiplier -1.0))))
    (:then_1
      (bind _clampedmana (CallFunction|GetClampedManaValues (+ (Variables|Default|Get_currentMana) (* Amount (LocalVariables|GetMultiplier)))))
      (Variables|Default|Set_currentMana _clampedmana))))

(fn GetClampedManaValues
  (params (IntendedMana :type Float%20%28double-precision%29))
  (return (Math|Float|Clamp(Float) IntendedMana 0.0 (Variables|Default|GetMaxMana))))

(fn GetManaValues
  (bind _maxmana (Variables|Default|GetMaxMana))
  (bind __currentmana (Variables|Default|Get_currentMana))
  (return (Math|Float|Truncate __currentmana) (Math|Float|Ceil _maxmana) (/ __currentmana _maxmana)))

(fn OnEnemyKilled
  (params (ManaEarned :type Integer))
  (CallFunction|ModifyManaValues true (Math|Conversions|ToFloat(Integer) ManaEarned))
  (Audio|PlaySound2D "/Game/Sound/SFX/UI/RecieveMana_Cue.RecieveMana_Cue" 1.0 1.0 0.0 0 0))

(fn Die
  (Game|OpenLevel(byName) "LoseScreen")
  (|CallParentFunction))

(fn GetAllSkills
  (for _array_element (Variables|/Game/Blueprints/Player/Skills/BP_PlayerSkillContainerComponent.BP_PlayerSkillContainerComponent_C|GetSkills (Variables|Default|GetBP_PlayerSkillContainerComponent))
    (bind _returnvalue (Game|AddComponentbyClass _array_element false))
    (Variables|/Game/Blueprints/Skills/BP_SK_PlayerSkillBase.BP_SK_PlayerSkillBase_C|SetPlayerController _returnvalue (Variables|Default|GetPlayerController))
    (Utilities|Array|AddUnique (Variables|Default|GetPlayerSkills) _returnvalue)))

(fn CheckSkillAvailable
  (params (SkillID :type Integer))
  (bind _available (Default|CheckManaAvailable (Utilities|Array|Get(acopy) (Variables|Default|GetPlayerSkills) SkillID) (Math|Float|Truncate (Variables|Default|Get_currentMana))))
  (return _available))

(fn OnSkillStart
  (params (SkillID :type Integer))
  (Default|OnSkillStart (Utilities|Array|Get(acopy) (Variables|Default|GetPlayerSkills) SkillID)))

(fn OnSkillEnd
  (params (SkillID :type Integer))
  (Default|OnSkillEnd (Utilities|Array|Get(acopy) (Variables|Default|GetPlayerSkills) SkillID)))

(fn GetCurrentAttacks
  (bind _returnvalue (Game|AddComponentbyClass (Variables|/Game/Blueprints/Player/Attacks/BP_PlayerAttackContainer.BP_PlayerAttackContainer_C|GetAutoAttackClass (Variables|Default|GetBP_PlayerAttackContainer))))
  (Variables|Default|SetAutoattack _returnvalue)
  (bind _returnvalue_2 (Game|AddComponentbyClass (Variables|/Game/Blueprints/Player/Attacks/BP_PlayerSwipeAttackContainer.BP_PlayerSwipeAttackContainer_C|GetSwipeAttackClass (Variables|Default|GetBP_PlayerSwipeAttackContainer))))
  (Variables|Default|SetSwipeAttack _returnvalue_2))

(fn GetAutoattack
  (bind _autoattack (Variables|Default|GetAutoattack))
  (return (Variables|/Game/Blueprints/Player/Attacks/Autoattack/BP_HeroAutoAttackBase.BP_HeroAutoAttackBase_C|GetAttackIcon _autoattack) (Variables|/Game/Blueprints/Player/Attacks/Autoattack/BP_HeroAutoAttackBase.BP_HeroAutoAttackBase_C|GetAttackName _autoattack)))

(fn GetSwipeAttack
  (bind _swipeattack (Variables|Default|GetSwipeAttack))
  (bind _cooldownperc (Default|GetCooldownValues _swipeattack))
  (return _cooldownperc (Variables|/Game/Blueprints/Player/Attacks/Swipeattack/BP_HeroSwipeAttackBase.BP_HeroSwipeAttackBase_C|GetAttackIcon _swipeattack) (Variables|/Game/Blueprints/Player/Attacks/Swipeattack/BP_HeroSwipeAttackBase.BP_HeroSwipeAttackBase_C|GetAttackName _swipeattack)))

(fn HandleHUDPosition
  (Class|UserWidget|SetPositioninViewport (Variables|Default|GetHUDHP) (.ScreenPosition (Class|GameplayStatics|ProjectWorldtoScreen (Game|GetPlayerController 0) (Transformation|GetWorldLocation (Variables|Character|GetMesh)) false)) true))