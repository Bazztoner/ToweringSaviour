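; Chain lightning autoattack projectile that hits its target, then jumps between nearby enemies with damage falling off per jump.
; BeginPlay spawns a lightning VFX actor toward the target, while an overlap component collects further enemies in EnemiesSorted.
; A looping timer retargets the bolt and damages the next list entry until MaxJumps, then destroys itself.
; SortTargetsByDistance is called before the timer, but its body is empty despite a distance comparator.
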(event OnComponentBeginOverlap(FurtherTargetsChecker)
  (params (OverlappedComponent :type Primitive%20Component%20Object%20Reference) (OtherActor :type Actor%20Object%20Reference) (OtherComp :type Primitive%20Component%20Object%20Reference) (OtherBodyIndex :type Integer) (bFromSweep :type Boolean) (SweepResult :type Hit%20Result%20Structure%20%28by%20ref%29))
  (bind _asbp_enemy_base (Utilities|Casting|CastToBP_EnemyBase OtherActor))
  (Utilities|Array|AddUnique (Variables|Default|GetEnemiesSorted) _asbp_enemy_base))

(event Custom|Attack
  (bind _lightningvfxobject (Variables|Default|GetLightningVFXObject))
  (bind _lightningvfxobject_2 (Variables|Default|GetLightningVFXObject))
  (if (< (Variables|Default|GetHitEnemies) (Variables|Default|GetMaxJumps))
    (CallFunction|SetLightningPositions)
    (bind _enemyfound (CallFunction|AttackEnemy))
    (Math|Integer|IncrementInt (Variables|Default|GetHitEnemies)
      (:%20%20
        (if (not _enemyfound)
          (Utilities|IsValid _lightningvfxobject_2
            (:Is%20Valid
              (Actor|DestroyActor _lightningvfxobject_2))))))
    (else
      (Utilities|FlowControl|Sequence
        (:then_0
          (Utilities|IsValid _lightningvfxobject
            (:Is%20Valid
              (Actor|DestroyActor _lightningvfxobject))))
        (:then_1
          (Actor|DestroyActor))))))

(event EventBeginPlay
  (Utilities|FlowControl|Sequence
    (:then_0
      (Utilities|IsValid (Variables|Default|GetEnemyTarget)
        (:Is%20Valid
          (Utilities|Array|AddUnique (Variables|Default|GetEnemiesSorted) (Variables|Default|GetEnemyTarget))
          (bind _returnvalue (Game|SpawnActorfromClass (Variables|Default|GetLightningVFXClass) (Transformation|GetActorTransform) "AlwaysSpawn" 0 0))
          (bind _output_get (Variables|Default|SetLightningVFXObject _returnvalue))
          (Default|SetPositions _output_get (.location (Transformation|GetActorTransform)) (Transformation|GetActorLocation (Variables|Default|GetEnemyTarget))))))
    (:then_1
      (Utilities|FlowControl|DelayUntilNextTick)
      (CallFunction|SortTargetsbyDistance)
      (Utilities|Time|SetTimerbyEvent (delegate Custom|Attack) (Variables|Default|GetHitDelay) true))))

(fn ConstructionScript)

(fn SortTargetsbyDistance)

(fn DistanceEnemyDelegate
  (params (A :type Actor%20Object%20Reference) (B :type Actor%20Object%20Reference))
  (bind _self self)
  (return (> (Transformation|GetDistanceTo A _self) (Transformation|GetDistanceTo B _self))))

(fn AttackEnemy
  (bind _enemiessorted (Variables|Default|GetEnemiesSorted))
  (bind _hitenemies (Variables|Default|GetHitEnemies))
  (bind _output (Utilities|Array|Get(acopy) _enemiessorted _hitenemies))
  (bind _returnvalue (Transformation|GetActorTransform _output))
  (bind _output_get (LocalVariables|SetEnemyToAttack _output))
  (Utilities|IsValid _output_get
    (:Is%20Valid
      (CallFunction|OnEnemyHit (.location _returnvalue))
      (Niagara|SpawnSystematLocation "/Game/Art/Particles/PS_LightningStruck.PS_LightningStruck" (.location _returnvalue) "0, 0, 0" "1.000000,1.000000,1.000000" true true "AutoRelease")
      (Game|Damage|ApplyDamage (LocalVariables|GetEnemyToAttack) (- (Variables|Default|GetDamage) (* (Variables|Default|GetDamageLostPerJump) (Variables|Default|GetHitEnemies))) 0 0)
      (return true))
    (:Is%20Not%20Valid
      (return false))))

(fn SetLightningPositions
  (bind _hitenemies (Variables|Default|GetHitEnemies))
  (bind _enemiessorted (Variables|Default|GetEnemiesSorted))
  (bind _lightningvfxobject (Variables|Default|GetLightningVFXObject))
  (bind _returnvalue (+ _hitenemies 1))
  (bind _output (Utilities|Array|Get(acopy) _enemiessorted _returnvalue))
  (if (< (Variables|Default|GetHitEnemies) (- (Variables|Default|GetMaxJumps) 1))
    (if (and (Utilities|IsValid (Utilities|Array|Get(acopy) (Variables|Default|GetEnemiesSorted) (Variables|Default|GetHitEnemies))) (Utilities|IsValid _output))
      (Utilities|IsValid _lightningvfxobject
        (:Is%20Valid
          (Default|SetNextTarget _lightningvfxobject (Transformation|GetActorLocation _output)))))))