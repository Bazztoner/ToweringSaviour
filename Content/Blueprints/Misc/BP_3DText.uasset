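; BP_3DText is a short-lived world text actor that shows a given string in a given color, then destroys itself.
; On BeginPlay it sets up the Text component and creates a dynamic instance of its material, without assigning it back to the component.
; The Lifetime timeline feeds Alpha to that instance as a scalar, though the parameter name is None, and destroys the actor when finished.
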(event EventBeginPlay
  (bind _text (Variables|Default|GetText))
  (bind _returnvalue (Rendering|Material|CreateDynamicMaterialInstance (Rendering|Material|GetMaterial (Variables|Default|GetText) 0) "None" "None" :!class /Script/Engine.KismetMaterialLibrary))
  (Variables|Default|SetMat _returnvalue)
  (Rendering|Components|TextRender|SetText _text (Variables|Default|GetDisplayText))
  (Rendering|Components|TextRender|SetTextRenderColor _text (Math|Conversions|ToColor(LinearColor) (Variables|Default|GetTextColor)))
  (bind _alpha (Timeline|Lifetime PlayFromStart)
    (:Update
      (Rendering|Material|SetScalarParameterValue (Variables|Default|GetMat) "None" _alpha :!class /Script/Engine.MaterialInstanceDynamic))
    (:Finished
      (Actor|DestroyActor))))

(event Collision|EventActorBeginOverlap
  (params (OtherActor :type Actor%20Object%20Reference)))

(event EventTick
  (params (DeltaSeconds :type Float%20%28single-precision%29)))

(fn ConstructionScript)