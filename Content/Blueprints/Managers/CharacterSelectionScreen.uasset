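; Manager for the character selection screen that tracks which hero is currently selected.
; On BeginPlay it sets a phone-sized portrait window, spawns Ninja, Mage and Demoman selection actors into AllHeroes, then creates the selection HUD with a self reference and UI-only input.
; ChangeHeroSelected cycles HeroIndex left or right with wraparound based on HeroAmount.
; GetSelectedHero returns the actor at that index.
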(event Custom|ChangeHeroSelected
  (params (Right :type Boolean))
  (if Right
    (if (>= (+ (Variables|Default|GetHeroIndex) 1) (Variables|Default|GetHeroAmount))
      (Variables|Default|SetHeroIndex 0)
      (else
        (Math|Integer|IncrementInt (Variables|Default|GetHeroIndex))))
    (elif (> (Variables|Default|GetHeroIndex) 0)
      (Math|Integer|DecrementInt (Variables|Default|GetHeroIndex))
      (else
        (Variables|Default|SetHeroIndex (- (Variables|Default|GetHeroAmount) 1))))))

(event EventBeginPlay
  (bind _returnvalue (Game|GetPlayerController 0))
  (Utilities|FlowControl|Sequence
    (:then_0
      (bind _returnvalue_2 (Settings|GetGameUserSettings))
      (Class|GameUserSettings|SetFullscreenMode _returnvalue_2 "Windowed")
      (Class|GameUserSettings|SetScreenResolution _returnvalue_2 (Utilities|Struct|MakeIntPoint 375 667))
      (Class|GameUserSettings|ApplyResolutionSettings _returnvalue_2 false)
      (bind _returnvalue_3 (Game|SpawnActorfromClass "/Game/Blueprints/Characters/CharacterSelection/BP_CharacterSelectionNinja.BP_CharacterSelectionNinja_C" (Math|Transform|MakeTransform "-500.000000,-500.000000,-500.000000" "0, 0, 0" "1.000000,1.000000,1.000000") "AlwaysSpawn" 0 0))
      (Utilities|Array|AddUnique (Variables|Default|GetAllHeroes) _returnvalue_3)
      (bind _returnvalue_4 (Game|SpawnActorfromClass "/Game/Blueprints/Characters/CharacterSelection/BP_CharacterSelectionMage.BP_CharacterSelectionMage_C" (Math|Transform|MakeTransform "-500.000000,-500.000000,-500.000000" "0, 0, 0" "1.000000,1.000000,1.000000") "AlwaysSpawn" 0 0))
      (Utilities|Array|AddUnique (Variables|Default|GetAllHeroes) _returnvalue_4)
      (bind _returnvalue_5 (Game|SpawnActorfromClass "/Game/Blueprints/Characters/CharacterSelection/BP_CharacterSelectionDemoman.BP_CharacterSelectionDemoman_C" (Math|Transform|MakeTransform "-500.000000,-500.000000,-500.000000" "0, 0, 0" "1.000000,1.000000,1.000000") "AlwaysSpawn" 0 0))
      (Utilities|Array|AddUnique (Variables|Default|GetAllHeroes) _returnvalue_5))
    (:then_1
      (Variables|/Script/Engine.PlayerController|SetbShowMouseCursor _returnvalue true)
      (bind _returnvalue_6 (UserInterface|CreateWidget "/Game/Blueprints/Widgets/CharacterSelection/HUD_NewCharaSelectScreen.HUD_NewCharaSelectScreen_C" _returnvalue self))
      (UserInterface|Viewport|AddtoViewport _returnvalue_6 0)
      (Input|SetInputModeUIOnly (Game|GetPlayerController 0) _returnvalue_6 "LockAlways"))))

(fn ConstructionScript)

(fn GetSelectedHero
  (return (Utilities|Array|Get(acopy) (Variables|Default|GetAllHeroes) (Variables|Default|GetHeroIndex))))